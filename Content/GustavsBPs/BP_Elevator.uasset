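; Elevator that carries the player into the next section, switching the music to level 2 on arrival.
; The first trigger pauses music once, opens the entry door, flips indicators to green and plays ambience.
; The second trigger passes mirror positions to the character's elevator mode, then once closes the door and fakes travel with delays and camera shake.
; OpenNextLevel then opens the exit door and starts level 2 music, without loading a map.
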(event `self.ReceiveBeginPlay`
  (bind _returnvalue (`GameplayStatics.GetActorOfClass` "/Game/GustavsBPs/BP_MusicManager.BP_MusicManager_C"))
  (set `self.MusicManager` _returnvalue))

(event `self.OpenDoorTrigget.OnComponentBeginOverlap`
  (params (OverlappedComponent :type "PrimitiveComponent Object Reference") (OtherActor :type "Actor Object Reference") (OtherComp :type "PrimitiveComponent Object Reference") (OtherBodyIndex :type Integer) (bFromSweep :type Boolean) (SweepResult :type "HitResult Structure (by ref)"))
  (bind _returnvalue (`SceneComponent.K2_GetComponentLocation` (`self.Door1`)))
  (cast `/Game/FirstPerson/Blueprints/BP_FirstPersonCharacter` OtherActor)
  (`/Engine/EditorBlueprintResources/StandardMacros.DoOnce` false
    (:`Completed`
      (bind _musicmanager (`self.MusicManager`)
        (:`then`
          (`/Game/GustavsBPs/BP_MusicManager.PauseAll` _musicmanager))
        (:`else`
          _))
      (`SkeletalMeshComponent.PlayAnimation` (`self.Door1`) "/Game/_GENERATED/gustavsjolund/Elevator_Anim_Elevqtor_Elevator_Open.Elevator_Anim_Elevqtor_Elevator_Open" false)
      (`PrimitiveComponent.SetCollisionEnabled` (`self.Collision1`) "NoCollision")
      (`SceneComponent.SetHiddenInGame` (`self.Green1`) false false)
      (`SceneComponent.SetHiddenInGame` (`self.Green`) false false)
      (`SceneComponent.SetHiddenInGame` (`self.Red1`) true false)
      (`SceneComponent.SetHiddenInGame` (`self.Red`) true false)
      (`GameplayStatics.PlaySoundAtLocation` "/Game/Audio/Sound/Elevator_OpenCat.Elevator_OpenCat" _returnvalue (struct) 1.0 1.0 0.0 null null null null)
      (`GameplayStatics.PlaySoundAtLocation` "/Game/Audio/Sound/Elevator_DiscoBallAmbiance.Elevator_DiscoBallAmbiance" _returnvalue (struct) 1.0 1.0 0.0 "/Game/Audio/Sound/SA_Spacial.SA_Spacial" null null null))))

(event `self.CloseDoorTrigger.OnComponentBeginOverlap`
  (params (OverlappedComponent :type "PrimitiveComponent Object Reference") (OtherActor :type "Actor Object Reference") (OtherComp :type "PrimitiveComponent Object Reference") (OtherBodyIndex :type Integer) (bFromSweep :type Boolean) (SweepResult :type "HitResult Structure (by ref)"))
  (bind _asbp_first_person_character (cast `/Game/FirstPerson/Blueprints/BP_FirstPersonCharacter` OtherActor))
  (`/Game/FirstPerson/Blueprints/BP_FirstPersonCharacter.Set Elevator Mode` _asbp_first_person_character (`SceneComponent.K2_GetComponentLocation` (`self.Pos`)) (`SceneComponent.K2_GetComponentLocation` (`self.Mirror`)))
  (`/Engine/EditorBlueprintResources/StandardMacros.DoOnce` false
    (:`Completed`
      (`SkeletalMeshComponent.PlayAnimation` (`self.Door1`) "/Game/_GENERATED/gustavsjolund/Elevator_Anim_Elevqtor_Elevator_Close.Elevator_Anim_Elevqtor_Elevator_Close" false)
      (`PrimitiveComponent.SetCollisionEnabled` (`self.Collision1`) "QueryAndPhysics")
      (`|ExecutionSequence`
        (:`then_0`
          (`KismetSystemLibrary.Delay` 3.0)
          (`GameplayStatics.PlayWorldCameraShake` "/Game/GustavsBPs/CS_Elevator.CS_Elevator_C" (`self.K2_GetActorLocation`) 100.0 1000.0)
          (`KismetSystemLibrary.Delay` 7.0)
          (`self.OpenNextLevel`))
        (:`then_1`
          (`GameplayStatics.PlaySoundAtLocation` "/Game/Audio/Sound/Elevator_OpenCat.Elevator_OpenCat" (`SceneComponent.K2_GetComponentLocation` (`self.Door1`)) (struct) 1.0 1.0 0.0 null null null null))))))

(event `OpenNextLevel`
  (`SkeletalMeshComponent.PlayAnimation` (`self.Door2`) "/Game/_GENERATED/gustavsjolund/Elevator_Anim_Elevqtor_Elevator_Open.Elevator_Anim_Elevqtor_Elevator_Open" false)
  (`PrimitiveComponent.SetCollisionEnabled` (`self.Collision2`) "NoCollision")
  (`GameplayStatics.PlaySoundAtLocation` "/Game/Audio/Sound/Elevator_OpenCat.Elevator_OpenCat" (`SceneComponent.K2_GetComponentLocation` (`self.Door2`)) (struct) 1.0 1.0 0.0 null null null null)
  (`KismetSystemLibrary.Delay` 2.0)
  (bind _musicmanager (`self.MusicManager`)
    (:`then`
      (`/Game/GustavsBPs/BP_MusicManager.PlayLevel2` _musicmanager))
    (:`else`)))

(fn `UserConstructionScript`)