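; BP_LilLamp is a lamp Blueprint that flickers while ShouldFlicker is true.
; Tick feeds a random short Delay, then stores a random Brightness and passes it to the Brightness material parameter on CeilingLights.
; The RectLight intensity comes from a separate, scaled random roll, so the light and the material brightness do not match.
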(event `self.ReceiveTick`
  (params (DeltaSeconds :type "Float (single-precision)"))
  (bind _returnvalue (`KismetMathLibrary.RandomFloatInRange` 0.0 10.0))
  (if (`self.ShouldFlicker`)
    (`KismetSystemLibrary.Delay` (`KismetMathLibrary.RandomFloatInRange` 0.0 0.5))
    (set `self.Brightness` _returnvalue)
    (`|ExecutionSequence`
      (:`then_0`
        (`LightComponent.SetIntensity` (`self.RectLight`) (* _returnvalue 1000.0)))
      (:`then_1`
        (`MeshComponent.SetScalarParameterValueOnMaterials` (`self.Ceiling_Lights`) "Brightness" (`self.Brightness`))))))

(fn `UserConstructionScript`)